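; Wild Pokémon encounter zone that rolls Route 2 encounters while the top-down player overlaps its box.
; A looping timer rolls with odds that rise after each failure, pausing on success or exit.
; A weighted map pick selects the species, matched to a Pokemon_Master_BP actor for random shininess, IVs and data-table level range.
; The result goes to the Game Instance through a save-encounter message.
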(event `SetEncounterArray`
  (if (== (`KismetMathLibrary.RandomIntegerInRange` 1 2) 1)
    (set `self.Is Shiny` true)
    (else
      (set `self.Is Shiny` false)))
  (bind _chosen_encounter (`self.RollEncounter`))
  (bind _outactors (`GameplayStatics.GetAllActorsOfClass` "/Game/Pokemon/Pokemons_Ready/Pokemon_Master_BP.Pokemon_Master_BP_C"))
  (for _array_element _outactors
    (bind _pokemoninfo (`/Game/Pokemon/Pokemons_Ready/Pokemon_Master_BP.PokemonInfo` _array_element))
    (bind (_pokedexlist _pokemonclass _name) (break `/Game/Pokemon/PokemonBaseInfo_Struct` _pokemoninfo))
    (if (== _chosen_encounter _name)
      (bind _pokemoninfostructout (`self.SetShiny` _pokemoninfo (`self.Is Shiny`)))
      (bind _structout (`self.RollIv's` (`/Game/Pokemon/Pokemons_Ready/Pokemon_Master_BP.Pokemon IVs` _array_element)))
      (bind (_pokemon_stat_out _pokemon_info_out) (`self.Roll Base Stat's` (`/Game/Pokemon/Pokemons_Ready/Pokemon_Master_BP.PokemonStats` _array_element) _pokemoninfostructout))
      (bind _output_get (set `/Game/Pokemon/Pokemons_Ready/Pokemon_Master_BP.PokemonInfo` _pokemon_info_out _array_element))
      (message `/Game/PokeWorldAdventure/Blueprints/InterfaceBPI.SaveEncounterInfo` (`GameplayStatics.GetGameInstance`) _pokemonclass _output_get _pokemon_stat_out _structout)
      (else
        (`KismetSystemLibrary.PrintString` "Hello")))))

(event `self.Box.OnComponentBeginOverlap`
  (params (OverlappedComponent :type "PrimitiveComponent Object Reference") (OtherActor :type "Actor Object Reference") (OtherComp :type "PrimitiveComponent Object Reference") (OtherBodyIndex :type Integer) (bFromSweep :type Boolean) (SweepResult :type "HitResult Structure (by ref)"))
  (cast `/Game/PokeWorldAdventure/Blueprints/BP_TopDownCharacter` OtherActor)
  (`KismetSystemLibrary.Delay` 1.0)
  (set `self.Inrange` false)
  (bind _returnvalue (`KismetSystemLibrary.K2_SetTimerDelegate` (delegate `RollForEncounter`) 0.5 true))
  (set `self.Spawn Timer` _returnvalue))

(event `self.Box.OnComponentEndOverlap`
  (params (OverlappedComponent :type "PrimitiveComponent Object Reference") (OtherActor :type "Actor Object Reference") (OtherComp :type "PrimitiveComponent Object Reference") (OtherBodyIndex :type Integer))
  (cast `/Game/PokeWorldAdventure/Blueprints/BP_TopDownCharacter` OtherActor)
  (`KismetSystemLibrary.Delay` 0.2)
  (set `self.Inrange` false)
  (`KismetSystemLibrary.K2_PauseTimerHandle` (`self.Spawn Timer`)))

(event `RollForEncounter`
  (if (`KismetMathLibrary.RandomBoolWithWeight` (+ 0.1 (* (`self.Times Roll Failed`) 0.05)))
    (set `self.Times Roll Failed` 0)
    (`KismetSystemLibrary.K2_PauseTimerHandle` (`self.Spawn Timer`))
    (`self.SetEncounterArray`)
    (else
      (`/Engine/EditorBlueprintResources/StandardMacros.IncrementInt` (`self.Times Roll Failed`)))))

(fn `Roll Base Stat's`
  (params (`Pokemon Stats` :type "/Game/Pokemon/PokemonBaseStat_Struct Structure") (`Pokemon Info` :type "/Game/Pokemon/PokemonBaseInfo_Struct Structure"))
  (returns (`Pokemon Stat Out` :type "/Game/Pokemon/PokemonBaseStat_Struct Structure") (`Pokemon Info Out` :type "/Game/Pokemon/PokemonBaseInfo_Struct Structure (by ref)"))
  (bind (_pokedexlist _pokemonclass _name _species _type1 _type2 _description _weight _height _sprite _moveslot1 _moveslot2 _moveslot3 _moveslot4 _currentlevel _maxlevel _evolutionlevel _isshiny) (break `/Game/Pokemon/PokemonBaseInfo_Struct` `Pokemon Info`))
  (bind _outrownames (`DataTableFunctionLibrary.GetDataTableRowNames` "/Game/Pokemon/Route2-EncounterDT.Route2-EncounterDT"))
  (for _array_element _outrownames
    (if (== _array_element _name)
      (bind _returnvalue (`|GetDataTableRow` "/Game/Pokemon/Route2-EncounterDT.Route2-EncounterDT" _array_element)
        (:`then`
          (bind (_pokemonname _typing1 _typing2 _minimumlevel _maximumlevel) (break `/Game/Pokemon/Encounter_Struct` _returnvalue))
          (bind _structout (setmembers `/Game/Pokemon/PokemonBaseInfo_Struct` :`StructRef` `Pokemon Info` :`Current Level` (`KismetMathLibrary.RandomIntegerInRange` _minimumlevel _maximumlevel) :`IsShiny` _isshiny))
          (return (struct) _structout))))))

(fn `RollEncounter`
  (returns (`Chosen Encounter` :type Name))
  (locals (SumofArray :type "Float (double-precision)") (Roll :type "Float (double-precision)"))
  (bind _roll (`local.Roll`))
  (bind _route2 (break `/Game/Pokemon/PossibleEncounters` (`self.PossibleEncounters`)))
  (set `local.SumofArray` 0.0)
  (bind _values (`BlueprintMapLibrary.Map_Values` (`.Route2_5_77F6E4644091836EC2E758BA9F43EBB6` (break `/Game/Pokemon/PossibleEncounters` (`self.PossibleEncounters`)))))
  (for _array_element _values
    (set `local.SumofArray` (+ _array_element (`local.SumofArray`))))
  (set `local.Roll` (`KismetMathLibrary.RandomFloatInRange` 0.0 (`local.SumofArray`)))
  (bind _keys (`BlueprintMapLibrary.Map_Keys` _route2))
  (for _array_element_2 _keys
    (bind _value (`BlueprintMapLibrary.Map_Find` _route2 _array_element_2))
    (if (>= _value _roll)
      (set `self.Chosen Encounter` _array_element_2)
      (break)
      (else
        (set `local.Roll` (- _roll _value)))))
  (return (`self.Chosen Encounter`)))

(fn `RollIv's`
  (params (`Pokemon_IV In` :type "/Game/Pokemon/Pokemon_IV_Struct Structure (by ref)"))
  (returns (StructOut :type "/Game/Pokemon/Pokemon_IV_Struct Structure (by ref)"))
  (bind _structout (setmembers `/Game/Pokemon/Pokemon_IV_Struct` :`StructRef` `Pokemon_IV In` :`HP` (`KismetMathLibrary.RandomIntegerInRange` 0 31) :`Attack` (`KismetMathLibrary.RandomIntegerInRange` 0 31) :`Defence` (`KismetMathLibrary.RandomIntegerInRange` 0 31) :`Speed` (`KismetMathLibrary.RandomIntegerInRange` 0 31) :`Accuracy` (`KismetMathLibrary.RandomIntegerInRange` 0 31) :`Sp.Defence` (`KismetMathLibrary.RandomIntegerInRange` 0 31) :`Sp.Attack` (`KismetMathLibrary.RandomIntegerInRange` 0 31)))
  (return _structout))

(fn `SetShiny`
  (params (PokemonInfo :type "/Game/Pokemon/PokemonBaseInfo_Struct Structure") (`Is Shiny` :type Boolean))
  (returns (PokemonInfoStructOut :type "/Game/Pokemon/PokemonBaseInfo_Struct Structure (by ref)"))
  (bind _structout (setmembers `/Game/Pokemon/PokemonBaseInfo_Struct` :`StructRef` PokemonInfo :`IsShiny` `Is Shiny`))
  (return _structout))

(fn `UserConstructionScript`)