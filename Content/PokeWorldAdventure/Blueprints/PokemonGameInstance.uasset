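; Game instance Blueprint for a Pokémon-style game that saves party and wild encounter data to save slots.
; SavePartyInfo writes the party and player transform into a new PartySaveGame in its own slot.
; SaveEncounterInfo writes the selected encounter with its info, stats and IVs into an EncounterSaveGame, then opens the grass battle level, so the save slot carries encounter data across the level change.
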(event `/Game/PokeWorldAdventure/Blueprints/InterfaceBPI.SavePartyInfo`
  (params (`Pokemon Party` :type "/Game/PokeWorldAdventure/Blueprints/Party_Struct Structure") (`Player Location` :type "Vector Structure") (`Player Rotation` :type "Rotator Structure"))
  (bind _returnvalue (`GameplayStatics.CreateSaveGameObject` "/Game/PokeWorldAdventure/Blueprints/PartySaveGame.PartySaveGame_C"))
  (set `/Game/PokeWorldAdventure/Blueprints/PartySaveGame.Pokemon Party` `Pokemon Party` _returnvalue)
  (set `/Game/PokeWorldAdventure/Blueprints/PartySaveGame.Player Location` `Player Location` _returnvalue)
  (set `/Game/PokeWorldAdventure/Blueprints/PartySaveGame.Player Rotation` `Player Rotation` _returnvalue)
  (bind _output_get (set `self.PartySave` _returnvalue))
  (`GameplayStatics.SaveGameToSlot` _output_get "PartySlot" 201))

(event `/Game/PokeWorldAdventure/Blueprints/InterfaceBPI.SaveEncounterInfo`
  (params (`Selected Encounter` :type "Actor Class Reference") (`Encounter Info` :type "/Game/Pokemon/PokemonBaseInfo_Struct Structure") (`Encounter Stats` :type "/Game/Pokemon/PokemonBaseStat_Struct Structure") (`Encounter IVS` :type "/Game/Pokemon/Pokemon_IV_Struct Structure"))
  (bind _returnvalue (`GameplayStatics.CreateSaveGameObject` "/Game/PokeWorldAdventure/Blueprints/EncounterSaveGame.EncounterSaveGame_C"))
  (set `/Game/PokeWorldAdventure/Blueprints/EncounterSaveGame.SelectedEncounter` `Selected Encounter` _returnvalue)
  (set `/Game/PokeWorldAdventure/Blueprints/EncounterSaveGame.PokemonInfo` `Encounter Info` _returnvalue)
  (set `/Game/PokeWorldAdventure/Blueprints/EncounterSaveGame.Pokemon Stats` `Encounter Stats` _returnvalue)
  (set `/Game/PokeWorldAdventure/Blueprints/EncounterSaveGame.Pokemon IVs` `Encounter IVS` _returnvalue)
  (bind _output_get (set `self.EncounterSave` _returnvalue))
  (`GameplayStatics.SaveGameToSlot` _output_get "EncounterSlot" 101)
  (`GameplayStatics.OpenLevel` "Grass_Battle_Level"))