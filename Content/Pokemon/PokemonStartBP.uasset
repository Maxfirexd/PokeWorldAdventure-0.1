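; Starter Pokemon pickup actor that lets the player choose a first Pokemon through an interaction.
; Entering its box enables input, finds the Pokemon_Master_BP actor matching its PokemonName and copies that info, stats, IVs and EVs into the character's CurrentPokemon.
; Interact opens the AcceptPokemon widget in UI-only mode with a cursor, or prints a message if the player already has one.
; Leaving the box disables input.
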(event `self.Box.OnComponentBeginOverlap`
  (params (OverlappedComponent :type "PrimitiveComponent Object Reference") (OtherActor :type "Actor Object Reference") (OtherComp :type "PrimitiveComponent Object Reference") (OtherBodyIndex :type Integer) (bFromSweep :type Boolean) (SweepResult :type "HitResult Structure (by ref)"))
  (cast `/Game/PokeWorldAdventure/Blueprints/BP_TopDownCharacter` OtherActor)
  (`self.EnableInput` (`GameplayStatics.GetPlayerController` 0))
  (bind _outactors (`GameplayStatics.GetAllActorsOfClass` "/Game/Pokemon/Pokemons_Ready/Pokemon_Master_BP.Pokemon_Master_BP_C"))
  (for _array_element _outactors
    (bind _pokemoninfo (`/Game/Pokemon/Pokemons_Ready/Pokemon_Master_BP.PokemonInfo` _array_element))
    (if (== (`self.Pokemon Name`) (`.Name_61_AA49424842DDE825871BB29194006E04` (break `/Game/Pokemon/PokemonBaseInfo_Struct` _pokemoninfo)))
      (bind _structout (setmembers `/Game/Pokemon/PokemonBaseInfo_Struct` :`StructRef` _pokemoninfo))
      (bind _asbp_top_down_character (cast `/Game/PokeWorldAdventure/Blueprints/BP_TopDownCharacter` (`GameplayStatics.GetPlayerCharacter` 0)))
      (set `/Game/PokeWorldAdventure/Blueprints/BP_TopDownCharacter.Current Pokemon` (make `/Game/Pokemon/PokemonBuild_Struct` _structout (`/Game/Pokemon/Pokemons_Ready/Pokemon_Master_BP.PokemonStats` _array_element) (`/Game/Pokemon/Pokemons_Ready/Pokemon_Master_BP.Pokemon IVs` _array_element) (`/Game/Pokemon/Pokemons_Ready/Pokemon_Master_BP.Pokemon EVs` _array_element)) _asbp_top_down_character))))

(event `self.Box.OnComponentEndOverlap`
  (params (OverlappedComponent :type "PrimitiveComponent Object Reference") (OtherActor :type "Actor Object Reference") (OtherComp :type "PrimitiveComponent Object Reference") (OtherBodyIndex :type Integer))
  (cast `/Game/PokeWorldAdventure/Blueprints/BP_TopDownCharacter` OtherActor)
  (`self.DisableInput` (`GameplayStatics.GetPlayerController` 0)))

(event `InputAction|Interact`
  (params (Key :type "Key Structure"))
  (bind _returnvalue (`GameplayStatics.GetPlayerController` 0))
  (:`Pressed`
    (bind _asbp_top_down_character (cast `/Game/PokeWorldAdventure/Blueprints/BP_TopDownCharacter` (`GameplayStatics.GetPlayerCharacter` 0)))
    (if (`/Game/PokeWorldAdventure/Blueprints/BP_TopDownCharacter.Has Pokemon?` _asbp_top_down_character)
      (`KismetSystemLibrary.PrintString` "Has Pokemon")
      (else
        (bind _returnvalue_2 (`|CreateWidget` "/Game/PokeWorldAdventure/Widgets/AcceptPokemon.AcceptPokemon_C"))
        (`UserWidget.AddToViewport` _returnvalue_2 0)
        (`WidgetBlueprintLibrary.SetInputMode_UIOnlyEx` _returnvalue _returnvalue_2)
        (set `PlayerController.bShowMouseCursor` true _returnvalue)))))

(fn `UserConstructionScript`)